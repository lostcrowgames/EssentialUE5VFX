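; Actor component that plays a staged construction effect, revealing its owner's building parts one at a time with sound.
; Start gathers static mesh components tagged "Cube", sorts them by display name, then hides them, optionally disabling collision and applying progress materials.
; A looping BuildTime timer shows each part and restores any controlled collision.
; After the last part, it plays a completion sound and attempts a final material swap at the incremented index.
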(event `Start`
  (`self.AddBuildingPartsToArray`))

(event `AddBuildingPartsToArray`
  (bind _tmapstringtostaticmesh (`self.TMapStringToStaticMesh`))
  ; Add building parts from parent to array
  (bind _output_get (set `self.Array` (`Actor.GetComponentsByTag` (`self.GetOwner`) "/Script/Engine.StaticMeshComponent" "Cube")))
  (for _array_element _output_get
    (`BlueprintMapLibrary.Map_Add` _tmapstringtostaticmesh (`KismetSystemLibrary.GetDisplayName` _array_element) _array_element)
    (bind _keys (`BlueprintMapLibrary.Map_Keys` _tmapstringtostaticmesh))
    (set `self.StringArray` _keys))
  (`KismetArrayLibrary.SortStringArray` (`self.StringArray`))
  (for _array_element_2 (`self.StringArray`)
    (`KismetArrayLibrary.Array_Add` (`self.ArraySorted`) (`BlueprintMapLibrary.Map_Find` (`self.TMapStringToStaticMesh`) _array_element_2)))
  (`self.HideBuildingParts`))

(event `HideBuildingParts`
  ; Make building parts invisible initially
  (for _array_element (`self.Array`)
    (`SceneComponent.SetVisibility` _array_element false true)
    (if (`self.ControlCollision`)
      (`PrimitiveComponent.SetCollisionEnabled` _array_element "NoCollision")
      (if (`self.SetCustomBuildingProgressMaterial`)
        (`PrimitiveComponent.SetMaterial` _array_element 0 "/Game/EssentialUE5FX/Assets/Materials/M_Transluscent_Orange.M_Transluscent_Orange")
        (`MeshComponent.SetOverlayMaterial` _array_element (`self.BuildingProgressMaterial`)))))
  (`self.StartBuildingEffect`))

(event `StartBuildingEffect`
  ; Set visibility on each building part
  (bind _returnvalue (`KismetSystemLibrary.K2_SetTimerDelegate` (delegate `MakeVisibile`) (`self.BuildTime`) true))
  (set `self.Timer` _returnvalue))

(event `MakeVisibile`
  (bind _output (`|GetArrayItem` (`self.ArraySorted`) (`self.Index`)))
  ; Set visibility on each building part
  (if (< (`self.Index`) (`KismetArrayLibrary.Array_Length` (`self.ArraySorted`)))
    (`SceneComponent.SetVisibility` _output true true)
    (`GameplayStatics.PlaySoundAtLocation` (`self.BuildingSound`) (`SceneComponent.RelativeLocation` _output) (struct) 1.0 1.0 0.0 null null null null)
    (if (`self.ControlCollision`)
      (`PrimitiveComponent.SetCollisionEnabled` _output "QueryAndPhysics"))
    (bind _result (`/Engine/EditorBlueprintResources/StandardMacros.IncrementInt` (`self.Index`))
      (:`  `
        ;; Play completed sound (or effect or w.e) when building is completed
        (if (== _result (`KismetArrayLibrary.Array_Length` (`self.ArraySorted`)))
          (`KismetSystemLibrary.Delay` 0.2)
          (`GameplayStatics.PlaySoundAtLocation` (`self.CompletedSound`) (`Actor.K2_GetActorLocation` (`self.GetOwner`)) (struct) 1.0 1.0 0.0 null null null null)
          (if (`self.SetCustomBuildingProgressMaterial`)
            (`PrimitiveComponent.SetMaterial` _output 0 (`self.FinalMaterial`))
            (`MeshComponent.SetOverlayMaterial` _output null)))))
    (else
      (`KismetSystemLibrary.K2_ClearAndInvalidateTimerHandle` (`self.Timer`)))))